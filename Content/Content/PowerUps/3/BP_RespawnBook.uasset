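; BP_RespawnBook is a respawn book power-up prop that spins and bobs in place; the file holds only this idle animation.
; BeginPlay caches the starting relative location of the Parent component.
; Each Tick advances separate rotation and bob timers, yawing the component at a fixed 90-degree roll and offsetting it along BobDirection with a cosine wave.
; No overlap, pickup or respawn logic is implemented here.
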(event EventBeginPlay
  (Variables|Default|SetStartRelativePosition (Variables|/Script/Engine.SceneComponent|GetRelativeLocation (Variables|Default|GetParent))))

(event Collision|EventActorBeginOverlap
  (params (OtherActor :type Actor%20Object%20Reference)))

(event EventTick
  (params (DeltaSeconds :type Float%20%28single-precision%29))
  (bind _output_get (Variables|Default|SetRotationTimer (+ (Variables|Default|GetRotationTimer) (* DeltaSeconds (Variables|Default|GetRotationSpeed)))))
  (Variables|Default|SetBobTimer (+ (Variables|Default|GetBobTimer) (* DeltaSeconds (Variables|Default|GetBobSpeed))))
  (Transformation|SetRelativeRotation (Variables|Default|GetParent) (Math|Rotator|MakeRotator 9e+01 0.0 _output_get) false false)
  (Transformation|SetRelativeLocation (Variables|Default|GetParent) (+ (Variables|Default|GetStartRelativePosition) (* (Variables|Default|GetBobDirection) (Math|Trig|Cos(Radians) (Variables|Default|GetBobTimer)))) false false))

(fn ConstructionScript)